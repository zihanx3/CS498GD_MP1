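; BP_Tunnel is a self-replacing tunnel segment with a rotating hole-wall obstacle for an endless tunnel game.
; Passing its trigger has TunnelSpawner spawn another tunnel, destroys this one and adds to BP_Player's score.
; Hitting the wall costs score and health, or on death refunds the point and shows restart; healthpacks restore random, capped health.
; RandomizeWall and RandomizeHealthpack vary meshes and rotation, usually also scattering the pack around a spawn point.
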(event `self.ReceiveBeginPlay`)

(event `self.ReceiveTick`
  (params (DeltaSeconds :type "Float (single-precision)"))
  (`SceneComponent.K2_AddLocalRotation` (`self.WallMesh`) (`KismetMathLibrary.MakeRotator` (* DeltaSeconds (`self.RotateSpeed`))) false false))

(event `self.TriggerZone.OnComponentBeginOverlap`
  (params (OverlappedComponent :type "PrimitiveComponent Object Reference") (OtherActor :type "Actor Object Reference") (OtherComp :type "PrimitiveComponent Object Reference") (OtherBodyIndex :type Integer) (bFromSweep :type Boolean) (SweepResult :type "HitResult Structure (by ref)"))
  ;[1 1 1] Add Score
  (bind _asbp_player (cast `/Game/InfiniteMatrix/Blueprints/BP_Player` OtherActor))
  (`/Game/InfiniteMatrix/Blueprints/BP_TunnelSpawner.SpawnTunnelAtSpawnPoint` (`self.TunnelSpawner`))
  (`self.K2_DestroyActor`)
  (set `/Game/InfiniteMatrix/Blueprints/BP_Player.score` (+ (`/Game/InfiniteMatrix/Blueprints/BP_Player.score` _asbp_player) 1) _asbp_player))

(event `self.WallMesh.OnComponentBeginOverlap`
  (params (OverlappedComponent :type "PrimitiveComponent Object Reference") (OtherActor :type "Actor Object Reference") (OtherComp :type "PrimitiveComponent Object Reference") (OtherBodyIndex :type Integer) (bFromSweep :type Boolean) (SweepResult :type "HitResult Structure (by ref)"))
  ;[1 1 1] Hit WallMesh
  (bind _asbp_player (cast `/Game/InfiniteMatrix/Blueprints/BP_Player` OtherActor))
  (set `/Game/InfiniteMatrix/Blueprints/BP_Player.score` (- (`/Game/InfiniteMatrix/Blueprints/BP_Player.score` _asbp_player) 1) _asbp_player)
  (bind _returnvalue (- (`/Game/InfiniteMatrix/Blueprints/BP_Player.health` _asbp_player) 0.2))
  (if (<= _returnvalue 0.0)
    (set `/Game/InfiniteMatrix/Blueprints/BP_Player.IsDead` true _asbp_player)
    (set `/Game/InfiniteMatrix/Blueprints/BP_Player.score` (+ (`/Game/InfiniteMatrix/Blueprints/BP_Player.score` _asbp_player) 1) _asbp_player)
    (`/Game/InfiniteMatrix/Blueprints/BP_Player.DisplayRestart` _asbp_player)
    (else
      (set `/Game/InfiniteMatrix/Blueprints/BP_Player.health` _returnvalue _asbp_player))))

(event `self.Healthpack.OnComponentBeginOverlap`
  (params (OverlappedComponent :type "PrimitiveComponent Object Reference") (OtherActor :type "Actor Object Reference") (OtherComp :type "PrimitiveComponent Object Reference") (OtherBodyIndex :type Integer) (bFromSweep :type Boolean) (SweepResult :type "HitResult Structure (by ref)"))
  ;[1 1 1] Add Healthpack
  (bind _asbp_player (cast `/Game/InfiniteMatrix/Blueprints/BP_Player` OtherActor))
  (bind _returnvalue (+ (`/Game/InfiniteMatrix/Blueprints/BP_Player.health` _asbp_player) (`KismetMathLibrary.RandomFloatInRange` 0.0 0.5)))
  (if (> _returnvalue 1.0)
    (set `/Game/InfiniteMatrix/Blueprints/BP_Player.health` 1.0 _asbp_player)
    (else
      (set `/Game/InfiniteMatrix/Blueprints/BP_Player.health` _returnvalue _asbp_player)))
  (`ActorComponent.K2_DestroyComponent` (`self.Healthpack`)))

(fn `RandomizeHealthpack`
  (params (SpawnPoint :type "Vector Structure"))
  (if (<= (`KismetMathLibrary.RandomIntegerInRange` 0 9) 8)
    (`StaticMeshComponent.SetStaticMesh` (`self.Healthpack`) (select `int` (`KismetMathLibrary.RandomIntegerInRange` 0 3) :`0` "/Game/InfiniteMatrix/Meshes/1M_Cube.1M_Cube" :`1` "/Game/InfiniteMatrix/Meshes/1M_Cube_Chamfer.1M_Cube_Chamfer" :`2` "/Game/InfiniteMatrix/Meshes/1M_Cube.1M_Cube" :`3` "/Game/InfiniteMatrix/Meshes/1M_Cube.1M_Cube" :!type "StaticMesh Object Reference"))
    (`SceneComponent.K2_AddLocalRotation` (`self.Healthpack`) (`KismetMathLibrary.MakeRotator` (`KismetMathLibrary.RandomFloatInRange` 0.0 360.0)) false false)
    (`SceneComponent.K2_SetWorldLocation` (`self.Healthpack`) (`KismetMathLibrary.RandomPointInBoundingBox` SpawnPoint (+ (0.0 0.0 0.0) (2000.0 200.0 200.0))) false false)))

(fn `RandomizeWall`
  (`StaticMeshComponent.SetStaticMesh` (`self.WallMesh`) (select `int` (`KismetMathLibrary.RandomIntegerInRange` 0 3) :`0` "/Game/InfiniteMatrix/Meshes/SM_Hole_01.SM_Hole_01" :`1` "/Game/InfiniteMatrix/Meshes/SM_Hole_02.SM_Hole_02" :`2` "/Game/InfiniteMatrix/Meshes/SM_Hole_03.SM_Hole_03" :`3` "/Game/InfiniteMatrix/Meshes/SM_Hole_04.SM_Hole_04" :!type "StaticMesh Object Reference"))
  (`SceneComponent.K2_AddLocalRotation` (`self.WallMesh`) (`KismetMathLibrary.MakeRotator` (`KismetMathLibrary.RandomFloatInRange` 0.0 360.0)) false false))

(fn `UserConstructionScript`)