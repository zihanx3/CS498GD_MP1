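; BP_Enemy is an obstacle enemy that damages BP_Player on contact.
; Its Box overlap event casts the other actor to BP_Player and subtracts a fixed amount from Health, with debug prints.
; RandomizeEnemy gives the Enemy component a random roll and teleport-free, non-swept move to a random point in a box offset along negative X from a supplied spawn location.
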(event `self.ReceiveActorBeginOverlap`
  (params (OtherActor :type "Actor Object Reference")))

(event `self.Box.OnComponentBeginOverlap`
  (params (OverlappedComponent :type "PrimitiveComponent Object Reference") (OtherActor :type "Actor Object Reference") (OtherComp :type "PrimitiveComponent Object Reference") (OtherBodyIndex :type Integer) (bFromSweep :type Boolean) (SweepResult :type "HitResult Structure (by ref)"))
  (`KismetSystemLibrary.PrintString` "Crash")
  (bind _asbp_player (cast `/Game/InfiniteMatrix/Blueprints/BP_Player` OtherActor))
  (`KismetSystemLibrary.PrintString` "Woops!")
  (set `/Game/InfiniteMatrix/Blueprints/BP_Player.health` (- (`/Game/InfiniteMatrix/Blueprints/BP_Player.health` _asbp_player) 0.4) _asbp_player))

(fn `RandomizeEnemy`
  (params (SpawnLocation :type "Vector Structure"))
  (`KismetSystemLibrary.PrintString` "Enemy Spawned")
  (`SceneComponent.K2_AddLocalRotation` (`self.Enemy`) (`KismetMathLibrary.MakeRotator` (`KismetMathLibrary.RandomFloatInRange` 0.0 360.0)) false false)
  (`SceneComponent.K2_SetWorldLocation` (`self.Enemy`) (`KismetMathLibrary.RandomPointInBoundingBox` (- SpawnLocation (500.0 0.0 0.0)) (+ (0.0 0.0 0.0) (300.0 100.0 100.0))) false false))

(fn `UserConstructionScript`)