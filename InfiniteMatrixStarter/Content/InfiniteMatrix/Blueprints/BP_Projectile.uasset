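; Player-fired projectile actor that destroys enemies on contact and awards score.
; Every tick it sets the projectile movement's initial and max speed from the player's forward speed plus fixed offsets, so it is meant to outpace the player.
; When its box overlaps a BP_Enemy, it increments the player's score, prints a debug hit message, and destroys both the enemy and itself.
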(event `self.ReceiveTick`
  (params (DeltaSeconds :type "Float (single-precision)"))
  (bind _projectilemovement (`self.ProjectileMovement`))
  (bind _asbp_player (cast `/Game/InfiniteMatrix/Blueprints/BP_Player` (`GameplayStatics.GetPlayerPawn` 0)))
  (bind _returnvalue (+ (`/Game/InfiniteMatrix/Blueprints/BP_Player.ForwardSpeed` _asbp_player) 1000.0))
  (set `ProjectileMovementComponent.InitialSpeed` _returnvalue _projectilemovement)
  (set `ProjectileMovementComponent.MaxSpeed` (+ _returnvalue 1000.0) _projectilemovement))

(event `self.Box.OnComponentBeginOverlap`
  (params (OverlappedComponent :type "PrimitiveComponent Object Reference") (OtherActor :type "Actor Object Reference") (OtherComp :type "PrimitiveComponent Object Reference") (OtherBodyIndex :type Integer) (bFromSweep :type Boolean) (SweepResult :type "HitResult Structure (by ref)"))
  (bind _asbp_enemy (cast `/Game/InfiniteMatrix/Blueprints/BP_Enemy` OtherActor))
  (bind _asbp_player (cast `/Game/InfiniteMatrix/Blueprints/BP_Player` (`GameplayStatics.GetPlayerPawn` 0)))
  (`KismetSystemLibrary.PrintString` "Hit +")
  (set `/Game/InfiniteMatrix/Blueprints/BP_Player.score` (+ (`/Game/InfiniteMatrix/Blueprints/BP_Player.score` _asbp_player) 1) _asbp_player)
  (`self.K2_DestroyActor` _asbp_enemy)
  (`self.K2_DestroyActor` self))

(fn `UserConstructionScript`)